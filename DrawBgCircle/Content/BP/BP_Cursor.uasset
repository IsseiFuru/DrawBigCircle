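; BP_Cursor is a cursor actor that removes itself based on cursor state held in the game instance.
; On Tick, when OneCursor's state is Remove and no circle is formed, it clears CursorList, then after a short delay restores the checkpoint list to its default and destroys itself.
; A completed circle keeps it alive until the next input, per the author's comment; TimeLimit is an empty stub.
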(event EventBeginPlay)

(event Collision|EventActorBeginOverlap
  (params (OtherActor :type Actor%20Object%20Reference)))

(event EventTick
  (params (DeltaSeconds :type Float%20%28single-precision%29))
  (bind _asbp_big_beautiful_circle_game_instance (CallFunction|GetGameInstanceRef))
  (switch string (.state (Variables|/Game/BP/BP_BBCircleGameInstance.BP_BBCircleGameInstance_C|GetOneCursor _asbp_big_beautiful_circle_game_instance))
    (:remove
      (if (not (Variables|/Game/BP/BP_BBCircleGameInstance.BP_BBCircleGameInstance_C|GetisCircle _asbp_big_beautiful_circle_game_instance)) ; 円が出来ていたら、次の入力まで消えない
        (Utilities|Array|Clear (Variables|/Game/BP/BP_BBCircleGameInstance.BP_BBCircleGameInstance_C|GetCursorList _asbp_big_beautiful_circle_game_instance))
        (Utilities|FlowControl|Delay 0.2)
        (Variables|/Game/BP/BP_BBCircleGameInstance.BP_BBCircleGameInstance_C|SetisCheckPointList _asbp_big_beautiful_circle_game_instance (Variables|/Game/BP/BP_BBCircleGameInstance.BP_BBCircleGameInstance_C|GetisDefaultCheckPointList _asbp_big_beautiful_circle_game_instance))
        (Actor|DestroyActor)))))

(fn ConstructionScript)

(fn TimeLimit)