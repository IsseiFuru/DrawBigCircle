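; Game mode for a circle-drawing game that scores how closely the player's drawn path follows a randomly placed circle marked by checkpoints.
; Tick reads cursor data from the game instance, spawns cursor and stroke actors, and accumulates radial error.
; On release, a nearly closed path through all checkpoints shows a score reduced by average error.
; Short directional strokes act as gestures that reset the round or toggle a cheat circle overlay.
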(event Custom|SpawnCursor
  (params (OneCursor :type F%20Cursor%20Structure))
  (bind _position (Utilities|Struct|BreakF_Cursor OneCursor))
  (bind _as_bp_big_beautiful_circle_game_instance (Variables|Default|GetAs%20BP%20Big%20Beautiful%20Circle%20Game%20Instance))
  ;[0.09399 0.8702 1] Spawn Cursor
  (bind _vector (CallFunction|FromMeasuredValuetoVector _position))
  (Game|SpawnActorfromClass "/Game/BP/BP_Cursor.BP_Cursor_C" (Math|Transform|MakeTransform _vector "0, 0, 0" "0.250000,0.250000,0.010000") "Undefined" 0 0)
  (CallFunction|SpawnStroke _position)
  (bind _position_2 (CallFunction|FromMeasuredValuetoVector _position))
  (bind _distance (CallFunction|TwoPointDistance _position_2 (Variables|/Game/BP/BP_BBCircleGameInstance.BP_BBCircleGameInstance_C|GetCenterPosition _as_bp_big_beautiful_circle_game_instance)))
  (Variables|/Game/BP/BP_BBCircleGameInstance.BP_BBCircleGameInstance_C|SetCenterDistance _as_bp_big_beautiful_circle_game_instance (+ (Math|Float|Absolute(Float) (- _distance (Variables|/Game/BP/BP_BBCircleGameInstance.BP_BBCircleGameInstance_C|GetRadius _as_bp_big_beautiful_circle_game_instance))) (Variables|/Game/BP/BP_BBCircleGameInstance.BP_BBCircleGameInstance_C|GetCenterDistance _as_bp_big_beautiful_circle_game_instance)))
  (Variables|/Game/BP/BP_BBCircleGameInstance.BP_BBCircleGameInstance_C|SetCursorCnt _as_bp_big_beautiful_circle_game_instance (+ (Variables|/Game/BP/BP_BBCircleGameInstance.BP_BBCircleGameInstance_C|GetCursorCnt _as_bp_big_beautiful_circle_game_instance) 1.0)))

(event Custom|InitialGameInstance
  ;[1 1 1] Initial Game Instance
  (bind _asbp_big_beautiful_circle_game_instance (CallFunction|GetGameInstanceRef))
  (bind _output_get (Variables|Default|SetAs%20BP%20Big%20Beautiful%20Circle%20Game%20Instance _asbp_big_beautiful_circle_game_instance))
  (Variables|/Game/BP/BP_BBCircleGameInstance.BP_BBCircleGameInstance_C|SetAddCursor _output_get "")
  (Variables|/Game/BP/BP_BBCircleGameInstance.BP_BBCircleGameInstance_C|SetRemoveCursor _output_get "")
  (Variables|/Game/BP/BP_BBCircleGameInstance.BP_BBCircleGameInstance_C|SetCenterPosition _output_get "(X=0.500000,Y=0.500000)")
  (Variables|/Game/BP/BP_BBCircleGameInstance.BP_BBCircleGameInstance_C|SetCenterDistance _output_get 0.0)
  (Variables|/Game/BP/BP_BBCircleGameInstance.BP_BBCircleGameInstance_C|SetScore _output_get 1e+02)
  (Variables|/Game/BP/BP_BBCircleGameInstance.BP_BBCircleGameInstance_C|SetisReset _output_get false))

(event Custom|Cheat%20Mode
  (bind _as_bp_big_beautiful_circle_game_instance (Variables|Default|GetAs%20BP%20Big%20Beautiful%20Circle%20Game%20Instance))
  (bind _centerposition (Variables|/Game/BP/BP_BBCircleGameInstance.BP_BBCircleGameInstance_C|GetCenterPosition _as_bp_big_beautiful_circle_game_instance))
  ;[1 1 1] Cheat Mode
  (if (Variables|/Game/BP/BP_BBCircleGameInstance.BP_BBCircleGameInstance_C|GetisCheat _as_bp_big_beautiful_circle_game_instance)
    (if (not (Utilities|IsValid (Variables|Default|GetDebug%20Circle%20Object)))
      (bind _returnvalue (Game|SpawnActorfromClass "/Game/BP/DebugCircle.DebugCircle_C" (Math|Transform|MakeTransform (Math|Vector|MakeVector 0.5 (.x _centerposition) (.y _centerposition)) "0, 0, 0" (Math|Conversions|ToVector(Float) (/ (Variables|/Game/BP/BP_BBCircleGameInstance.BP_BBCircleGameInstance_C|GetRadius _as_bp_big_beautiful_circle_game_instance) 5e+01))) "Undefined" 0 0))
      (Variables|Default|SetDebug%20Circle%20Object _returnvalue))
    (elif (Utilities|IsValid (Variables|Default|GetDebug%20Circle%20Object))
      (Actor|DestroyActor (Variables|Default|GetDebug%20Circle%20Object)))))

(event Custom|SpawnCheckPoint
  ;[0.09399 0.8702 1] SpawnCheckPoint
  (CallFunction|SetCircle)
  (CallFunction|SetCheckPointPosition)
  (for (_array_element _array_index) (Variables|/Game/BP/BP_BBCircleGameInstance.BP_BBCircleGameInstance_C|GetCheckPointPosition (Variables|Default|GetAs%20BP%20Big%20Beautiful%20Circle%20Game%20Instance))
    (Game|SpawnActorfromClass "/Game/BP/BP_CheckPoint.BP_CheckPoint_C" (Math|Transform|MakeTransform _array_element "0, 0, 0" "0.350000,0.350000,0.030000") "Undefined" 0 _array_index 0)))

(event Custom|CheckCircle
  (bind _as_bp_big_beautiful_circle_game_instance (Variables|Default|GetAs%20BP%20Big%20Beautiful%20Circle%20Game%20Instance))
  ;[1 1 1] Check Circle
  (if (and (Utilities|Enum|Equal(Enum) (.state (Variables|/Game/BP/BP_BBCircleGameInstance.BP_BBCircleGameInstance_C|GetOneCursor _as_bp_big_beautiful_circle_game_instance)) "remove") (== (Variables|/Game/BP/BP_BBCircleGameInstance.BP_BBCircleGameInstance_C|GetBpEpDistance _as_bp_big_beautiful_circle_game_instance) 0.0))
    (CallFunction|ResetCheck)
    (bind _distance (CallFunction|TwoPointDistance (Variables|/Game/BP/BP_BBCircleGameInstance.BP_BBCircleGameInstance_C|GetAddCursor _as_bp_big_beautiful_circle_game_instance) (Variables|/Game/BP/BP_BBCircleGameInstance.BP_BBCircleGameInstance_C|GetRemoveCursor _as_bp_big_beautiful_circle_game_instance)))
    (bind _output_get (Variables|/Game/BP/BP_BBCircleGameInstance.BP_BBCircleGameInstance_C|SetBpEpDistance _as_bp_big_beautiful_circle_game_instance _distance))
    (Variables|/Game/BP/BP_BBCircleGameInstance.BP_BBCircleGameInstance_C|SetAddCursor _as_bp_big_beautiful_circle_game_instance "")
    (if (<= _output_get 0.1)
      (if (Utilities|Array|Identical (Variables|/Game/BP/BP_BBCircleGameInstance.BP_BBCircleGameInstance_C|GetisCheckPointList _as_bp_big_beautiful_circle_game_instance) (Variables|/Game/BP/BP_BBCircleGameInstance.BP_BBCircleGameInstance_C|GetisThroughCheckPointList _as_bp_big_beautiful_circle_game_instance))
        (Variables|/Game/BP/BP_BBCircleGameInstance.BP_BBCircleGameInstance_C|SetisCircle _as_bp_big_beautiful_circle_game_instance true)
        (CallFunction|ShowScore)))))

(event Custom|Show%20Score
  (bind _as_bp_big_beautiful_circle_game_instance (Variables|Default|GetAs%20BP%20Big%20Beautiful%20Circle%20Game%20Instance))
  ;[1 1 1] Show Score
  (if (>= (- (Variables|/Game/BP/BP_BBCircleGameInstance.BP_BBCircleGameInstance_C|GetScore _as_bp_big_beautiful_circle_game_instance) (/ (Variables|/Game/BP/BP_BBCircleGameInstance.BP_BBCircleGameInstance_C|GetCenterDistance _as_bp_big_beautiful_circle_game_instance) (Variables|/Game/BP/BP_BBCircleGameInstance.BP_BBCircleGameInstance_C|GetCursorCnt _as_bp_big_beautiful_circle_game_instance))) 0.0)
    (Variables|/Game/BP/BP_BBCircleGameInstance.BP_BBCircleGameInstance_C|SetScore _as_bp_big_beautiful_circle_game_instance (- (Variables|/Game/BP/BP_BBCircleGameInstance.BP_BBCircleGameInstance_C|GetScore _as_bp_big_beautiful_circle_game_instance) (/ (Variables|/Game/BP/BP_BBCircleGameInstance.BP_BBCircleGameInstance_C|GetCenterDistance _as_bp_big_beautiful_circle_game_instance) (Variables|/Game/BP/BP_BBCircleGameInstance.BP_BBCircleGameInstance_C|GetCursorCnt _as_bp_big_beautiful_circle_game_instance))))
    (else
      (Variables|/Game/BP/BP_BBCircleGameInstance.BP_BBCircleGameInstance_C|SetScore _as_bp_big_beautiful_circle_game_instance 0.0)))
  (UserInterface|Viewport|AddtoViewport (Variables|Default|GetWBP_Score) 0))

(event Custom|Set%20CheckPoint%20Position
  (bind _returnvalue (Math|Random|RandomFloatinRange 0.0 3.6e+02))
  (bind _as_bp_big_beautiful_circle_game_instance (Variables|Default|GetAs%20BP%20Big%20Beautiful%20Circle%20Game%20Instance))
  (bind _debug_circle_object (Variables|Default|GetDebug%20Circle%20Object))
  (bind _checkpointposition (Variables|/Game/BP/BP_BBCircleGameInstance.BP_BBCircleGameInstance_C|GetCheckPointPosition _as_bp_big_beautiful_circle_game_instance))
  (bind _radius (Variables|/Game/BP/BP_BBCircleGameInstance.BP_BBCircleGameInstance_C|GetRadius _as_bp_big_beautiful_circle_game_instance))
  (bind _centerposition (Variables|/Game/BP/BP_BBCircleGameInstance.BP_BBCircleGameInstance_C|GetCenterPosition _as_bp_big_beautiful_circle_game_instance))
  ;[1 1 1] Set CheckPoint Position
  (if (Utilities|IsValid _debug_circle_object)
    (Actor|DestroyActor _debug_circle_object))
  (for (_ _array_index) _checkpointposition
    (Utilities|Array|SetArrayElem _checkpointposition _array_index (Math|Vector|MakeVector 0.1 (+ (* (Math|Trig|Cos(Radians) _returnvalue) _radius) (.x _centerposition)) (+ (.y _centerposition) (* _radius (Math|Trig|Sin(Radians) _returnvalue)))))
    (Variables|/Game/BP/BP_BBCircleGameInstance.BP_BBCircleGameInstance_C|SetisReset _as_bp_big_beautiful_circle_game_instance false)))

(event Custom|Spawn%20Stroke
  (params (OneCursorPosition :type Vector%202D%20Structure))
  (bind _as_bp_big_beautiful_circle_game_instance (Variables|Default|GetAs%20BP%20Big%20Beautiful%20Circle%20Game%20Instance))
  (bind _cursorlist (Variables|/Game/BP/BP_BBCircleGameInstance.BP_BBCircleGameInstance_C|GetCursorList _as_bp_big_beautiful_circle_game_instance))
  (bind _returnvalue (Utilities|Array|LastIndex _cursorlist))
  (bind _output (Utilities|Array|Get(acopy) _cursorlist _returnvalue))
  ;[0.09399 0.8702 1] Spawn Stroke
  (if (!= (Utilities|Array|Length _cursorlist) 0)
    (Variables|/Game/BP/BP_BBCircleGameInstance.BP_BBCircleGameInstance_C|SetVector2DSum _as_bp_big_beautiful_circle_game_instance (+ (- OneCursorPosition _output) (Variables|/Game/BP/BP_BBCircleGameInstance.BP_BBCircleGameInstance_C|GetVector2DSum _as_bp_big_beautiful_circle_game_instance)))
    (bind (_position _rotation _scale) (CallFunction|GetStrokeTransform _output OneCursorPosition))
    (bind _vector (CallFunction|FromMeasuredValuetoVector _position))
    (Game|SpawnActorfromClass "/Game/BP/BP_Stroke.BP_Stroke_C" (Math|Transform|MakeTransform _vector _rotation _scale) "Undefined" 0 0))
  (Utilities|Array|Add _cursorlist OneCursorPosition))

(event Custom|Set%20Circle
  (bind _as_bp_big_beautiful_circle_game_instance (Variables|Default|GetAs%20BP%20Big%20Beautiful%20Circle%20Game%20Instance))
  ;[1 1 1] Set Circle
  (bind _output_get (Variables|/Game/BP/BP_BBCircleGameInstance.BP_BBCircleGameInstance_C|SetCenterPosition _as_bp_big_beautiful_circle_game_instance (Math|Vector2D|MakeVector2D (Math|Random|RandomFloatinRange -3e+02 3e+02) (Math|Random|RandomFloatinRange -6e+01 6e+01))))
  (Variables|/Game/BP/BP_BBCircleGameInstance.BP_BBCircleGameInstance_C|SetRadius _as_bp_big_beautiful_circle_game_instance (Math|Random|RandomFloatinRange 2e+02 3e+02)))

(event Custom|ResetCheck
  (bind _as_bp_big_beautiful_circle_game_instance (Variables|Default|GetAs%20BP%20Big%20Beautiful%20Circle%20Game%20Instance))
  (bind _vector2dsum (Variables|/Game/BP/BP_BBCircleGameInstance.BP_BBCircleGameInstance_C|GetVector2DSum _as_bp_big_beautiful_circle_game_instance))
  (bind _cursorlist (Variables|/Game/BP/BP_BBCircleGameInstance.BP_BBCircleGameInstance_C|GetCursorList _as_bp_big_beautiful_circle_game_instance))
  (bind _vector2dsum_2 (Variables|/Game/BP/BP_BBCircleGameInstance.BP_BBCircleGameInstance_C|GetVector2DSum _as_bp_big_beautiful_circle_game_instance))
  (bind _returnvalue (Utilities|Array|Length _cursorlist))
  ;[1 1 1] Reset Check
  (if (and (<= _returnvalue 20) (> _returnvalue 8))
    (if (and (<= (.x _vector2dsum) -0.05) (>= (.y _vector2dsum) 0.1))
      (Variables|/Game/BP/BP_BBCircleGameInstance.BP_BBCircleGameInstance_C|SetisReset _as_bp_big_beautiful_circle_game_instance true)
      (elif (and (>= (.x _vector2dsum_2) 0.05) (<= (.y _vector2dsum_2) -0.1))
        (if (Variables|/Game/BP/BP_BBCircleGameInstance.BP_BBCircleGameInstance_C|GetisCheat _as_bp_big_beautiful_circle_game_instance)
          (Variables|/Game/BP/BP_BBCircleGameInstance.BP_BBCircleGameInstance_C|SetisCheat _as_bp_big_beautiful_circle_game_instance false)
          (else
            (Variables|/Game/BP/BP_BBCircleGameInstance.BP_BBCircleGameInstance_C|SetisCheat _as_bp_big_beautiful_circle_game_instance true)))))))

(event EventBeginPlay
  (CallFunction|InitialGameInstance)
  (bind _returnvalue (UserInterface|CreateWidget "/Game/UI/WBP_Score.WBP_Score_C"))
  (Variables|Default|SetWBP_Score _returnvalue)
  (CallFunction|SpawnCheckPoint))

(event EventTick
  (params (DeltaSeconds :type Float%20%28single-precision%29))
  ;[1 1 1] Tick
  (bind _asbp_big_beautiful_circle_game_instance (CallFunction|GetGameInstanceRef))
  (CallFunction|CheatMode)
  (if (Variables|/Game/BP/BP_BBCircleGameInstance.BP_BBCircleGameInstance_C|GetisReset _asbp_big_beautiful_circle_game_instance)
    (CallFunction|SpawnCheckPoint))
  ;;[1 1 1] Check for differences from Before Cursror List
  (if (Utilities|Operators|EqualEqual (.position (Variables|/Game/BP/BP_BBCircleGameInstance.BP_BBCircleGameInstance_C|GetBeforeOneCursor _asbp_big_beautiful_circle_game_instance)) (.Position (Utilities|Struct|BreakF_Cursor (Variables|/Game/BP/BP_BBCircleGameInstance.BP_BBCircleGameInstance_C|GetOneCursor _asbp_big_beautiful_circle_game_instance))) 0.0)
    _
    (else
      (Variables|/Game/BP/BP_BBCircleGameInstance.BP_BBCircleGameInstance_C|SetBeforeOneCursor _asbp_big_beautiful_circle_game_instance (Variables|/Game/BP/BP_BBCircleGameInstance.BP_BBCircleGameInstance_C|GetOneCursor _asbp_big_beautiful_circle_game_instance))
      (Widget|RemovefromParent (Variables|Default|GetWBP_Score))
      (CallFunction|SpawnCursor (Variables|/Game/BP/BP_BBCircleGameInstance.BP_BBCircleGameInstance_C|GetOneCursor _asbp_big_beautiful_circle_game_instance))))
  (CallFunction|CheckCircle))

(fn ConstructionScript)