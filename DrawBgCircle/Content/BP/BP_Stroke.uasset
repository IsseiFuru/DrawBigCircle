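; BP_Stroke is a stroke mesh actor in what appears to be a cursor-drawn circle game, managing its color and lifetime.
; Each Tick it reads the cursor state, circle flag and score from the Game Instance.
; Without a circle, it blackens and destroys itself on Add, or destroys itself after a short Delay on Remove.
; A completed circle persists, turning gold on Remove if the score is high enough.
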(event EventBeginPlay)

(event Collision|EventActorBeginOverlap
  (params (OtherActor :type Actor%20Object%20Reference)))

(event EventTick
  (params (DeltaSeconds :type Float%20%28single-precision%29))
  (bind _asbp_big_beautiful_circle_game_instance (CallFunction|GetGameInstanceRef))
  (switch string (.state (Variables|/Game/BP/BP_BBCircleGameInstance.BP_BBCircleGameInstance_C|GetOneCursor _asbp_big_beautiful_circle_game_instance))
    (:add
      (if (not (Variables|/Game/BP/BP_BBCircleGameInstance.BP_BBCircleGameInstance_C|GetisCircle _asbp_big_beautiful_circle_game_instance))
        (Rendering|Material|SetMaterial (Variables|Default|GetStaticMesh) 0 "/Game/Material/M_Black.M_Black")
        (Actor|DestroyActor :!label _label)))
    (:remove
      (if (Variables|/Game/BP/BP_BBCircleGameInstance.BP_BBCircleGameInstance_C|GetisCircle _asbp_big_beautiful_circle_game_instance) ; 円が出来ていたら、次の入力まで消えない
        (if (>= (Variables|/Game/BP/BP_BBCircleGameInstance.BP_BBCircleGameInstance_C|GetScore _asbp_big_beautiful_circle_game_instance) 9e+01)
          (Rendering|Material|SetMaterial (Variables|Default|GetStaticMesh) 0 "/Game/Material/Gold.Gold"))
        (else
          (Utilities|FlowControl|Delay 0.2)
          (goto _label))))))

(fn ConstructionScript)