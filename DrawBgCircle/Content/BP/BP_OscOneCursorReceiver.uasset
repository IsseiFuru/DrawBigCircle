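; Receives single-cursor input over OSC and publishes it to the game instance.
; On BeginPlay it starts an OSC server on port 50000, then parses each bundled message into an FCursor of state, session ID and XY position.
; Only session 0 is stored; Add records the start position and resets circle, checkpoint, distance, score and count state, while Remove records the end position.
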(event Custom|OscMessageAnalysis
  (params (Bundle :type OSC%20Bundle%20Structure%20%28by%20ref%29) (IPAddress :type String) (Port :type Integer))
  (bind _returnvalue (Class|OSCManager|GetMessagesfromBundle Bundle))
  (for _array_element _returnvalue
    (bind _f_cursol (CallFunction|FillterOscAnalysis _array_element))
    (if (== (.SessionID (Utilities|Struct|BreakF_Cursor _f_cursol)) 0)
      (bind _asbp_big_beautiful_circle_game_instance (CallFunction|GetGameInstanceRef))
      (Variables|/Game/BP/BP_BBCircleGameInstance.BP_BBCircleGameInstance_C|SetOneCursor _asbp_big_beautiful_circle_game_instance _f_cursol)
      (switch string (.State (Utilities|Struct|BreakF_Cursor _f_cursol))
        (:add
          (CallFunction|ResetGameInstance)
          (Variables|/Game/BP/BP_BBCircleGameInstance.BP_BBCircleGameInstance_C|SetAddCursor _asbp_big_beautiful_circle_game_instance (.Position (Utilities|Struct|BreakF_Cursor _f_cursol))))
        (:remove
          (Variables|/Game/BP/BP_BBCircleGameInstance.BP_BBCircleGameInstance_C|SetRemoveCursor _asbp_big_beautiful_circle_game_instance (.Position (Utilities|Struct|BreakF_Cursor _f_cursol))))))))

(event EventBeginPlay
  (bind _returnvalue (Class|OSCManager|CreateOSCServer "0.0.0.0" 50000 false true "" self))
  (EventDispatchers|BindEventtoOnOscBundleReceived _returnvalue (delegate Custom|OscMessageAnalysis)))

(fn ConstructionScript)

(fn FillterOscAnalysis
  (params (OscMessage :type OSC%20Message%20Structure%20%28by%20ref%29))
  (Utilities|FlowControl|Sequence
    (:then_0
      (bind _value (Class|OSCManager|GetString OscMessage))
      (LocalVariables|SetState _value)
      (bind _value_2 (Class|OSCManager|GetInt32 OscMessage 1))
      (LocalVariables|SetSessionID _value_2))
    (:then_1
      (bind _value_3 (Class|OSCManager|GetFloat OscMessage 2))
      (LocalVariables|SetX _value_3)
      (bind _value_4 (Class|OSCManager|GetFloat OscMessage 3))
      (LocalVariables|SetY _value_4))
    (:then_2
      (return (Utilities|Struct|MakeF_Cursor (LocalVariables|GetState) (LocalVariables|GetSessionID) (Math|Vector2D|MakeVector2D (LocalVariables|GetX) (LocalVariables|GetY)))))))

(fn ResetGameInstance
  (bind _asbp_big_beautiful_circle_game_instance (CallFunction|GetGameInstanceRef))
  (Variables|/Game/BP/BP_BBCircleGameInstance.BP_BBCircleGameInstance_C|SetisCircle _asbp_big_beautiful_circle_game_instance false)
  (Variables|/Game/BP/BP_BBCircleGameInstance.BP_BBCircleGameInstance_C|SetisCheckPointList _asbp_big_beautiful_circle_game_instance (Variables|/Game/BP/BP_BBCircleGameInstance.BP_BBCircleGameInstance_C|GetisDefaultCheckPointList _asbp_big_beautiful_circle_game_instance))
  (Variables|/Game/BP/BP_BBCircleGameInstance.BP_BBCircleGameInstance_C|SetBpEpDistance _asbp_big_beautiful_circle_game_instance 0.0)
  (Variables|/Game/BP/BP_BBCircleGameInstance.BP_BBCircleGameInstance_C|SetCenterDistance _asbp_big_beautiful_circle_game_instance 0.0)
  (Variables|/Game/BP/BP_BBCircleGameInstance.BP_BBCircleGameInstance_C|SetScore _asbp_big_beautiful_circle_game_instance 1e+02)
  (Variables|/Game/BP/BP_BBCircleGameInstance.BP_BBCircleGameInstance_C|SetCursorCnt _asbp_big_beautiful_circle_game_instance 0.0)
  (return))