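; BP_Reset is an overlap-triggered reset button actor that flags a reset in the game instance.
; On begin overlap, guarded by IsHover, it sets the ResetBtnVector parameter in MPC_GlobalParams to a hover value and sets IsReset to true on the game instance.
; On end overlap it clears IsHover and restores the button color.
; It never clears IsReset or performs the reset itself.
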(event EventBeginPlay)

(event Collision|EventActorBeginOverlap
  (params (OtherActor :type Actor%20Object%20Reference))
  (if (not (Variables|Default|GetisHover))
    (Variables|Default|SetisHover true)
    (Rendering|Material|SetVectorParameterValue "/Game/Material/MPC_GlobalParams.MPC_GlobalParams" "ResetBtnVector" (Variables|Default|GetHover%20Value) :!class /Script/Engine.KismetMaterialLibrary)
    (bind _asbp_big_beautiful_circle_game_instance (CallFunction|GetGameInstanceRef))
    (Variables|/Game/BP/BP_BBCircleGameInstance.BP_BBCircleGameInstance_C|SetisReset _asbp_big_beautiful_circle_game_instance true)))

(event EventTick
  (params (DeltaSeconds :type Float%20%28single-precision%29)))

(event Collision|EventActorEndOverlap
  (params (OtherActor :type Actor%20Object%20Reference))
  (Variables|Default|SetisHover false)
  (Rendering|Material|SetVectorParameterValue "/Game/Material/MPC_GlobalParams.MPC_GlobalParams" "ResetBtnVector" (Variables|Default|GetBtn%20Color%20Value) :!class /Script/Engine.KismetMaterialLibrary))

(fn ConstructionScript)