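; BP_CheckPoint is a numbered checkpoint actor that records in the game instance when its sphere is overlapped.
; BeginPlay reads its saved passed state by CheckPointNumber, and any overlap sets that array entry and applies the passed material.
; Tick destroys the actor while the game instance's IsReset flag is set, otherwise restoring the default material whenever the checkpoint list matches the default list.
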(event OnComponentBeginOverlap(Sphere)
  (params (OverlappedComponent :type Primitive%20Component%20Object%20Reference) (OtherActor :type Actor%20Object%20Reference) (OtherComp :type Primitive%20Component%20Object%20Reference) (OtherBodyIndex :type Integer) (bFromSweep :type Boolean) (SweepResult :type Hit%20Result%20Structure%20%28by%20ref%29))
  (bind _asbp_big_beautiful_circle_game_instance (CallFunction|GetGameInstanceRef))
  (Utilities|Array|SetArrayElem (Variables|/Game/BP/BP_BBCircleGameInstance.BP_BBCircleGameInstance_C|GetisCheckPointList _asbp_big_beautiful_circle_game_instance) (Variables|Default|GetCheckPointNumber) true)
  (Rendering|Material|SetMaterial (Variables|Default|GetSphere) 0 "/Game/Material/M_ThroughCheckPoint.M_ThroughCheckPoint"))

(event EventBeginPlay
  (bind _asbp_big_beautiful_circle_game_instance (CallFunction|GetGameInstanceRef))
  (Variables|Default|SetisThroughCheckPoint (Utilities|Array|Get(acopy) (Variables|/Game/BP/BP_BBCircleGameInstance.BP_BBCircleGameInstance_C|GetisCheckPointList _asbp_big_beautiful_circle_game_instance) (Variables|Default|GetCheckPointNumber))))

(event EventTick
  (params (DeltaSeconds :type Float%20%28single-precision%29))
  (bind _asbp_big_beautiful_circle_game_instance (CallFunction|GetGameInstanceRef))
  (if (Variables|/Game/BP/BP_BBCircleGameInstance.BP_BBCircleGameInstance_C|GetisReset _asbp_big_beautiful_circle_game_instance)
    (Actor|DestroyActor)
    (elif (Utilities|Array|Identical (Variables|/Game/BP/BP_BBCircleGameInstance.BP_BBCircleGameInstance_C|GetisDefaultCheckPointList _asbp_big_beautiful_circle_game_instance) (Variables|/Game/BP/BP_BBCircleGameInstance.BP_BBCircleGameInstance_C|GetisCheckPointList _asbp_big_beautiful_circle_game_instance))
      (Rendering|Material|SetMaterial (Variables|Default|GetSphere) 0 "/Game/Material/M_CheckPoint.M_CheckPoint"))))

(fn ConstructionScript)