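; Game mode for a circle-drawing game that traces cursor input, validates the finished stroke as a circle and prints a score.
; BeginPlay resets shared Game Instance state and spawns numbered checkpoint actors.
; Tick spawns a cursor actor whenever the position changes, accumulating its deviation from the target radius.
; On cursor removal, a small start-to-end gap plus matching checkpoint lists confirms the circle, with accumulated deviation lowering the score.
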(event Custom|SpawnCursor
  (params (OneCursor :type F%20Cursor%20Structure))
  (bind _position (Utilities|Struct|BreakF_Cursor OneCursor))
  (bind _as_bp_big_beautiful_circle_game_instance (Variables|Default|GetAs%20BP%20Big%20Beautiful%20Circle%20Game%20Instance))
  ;[1 1 1] Spawn Cursor
  (bind _vector (CallFunction|FromMeasuredValuetoVector _position))
  (Game|SpawnActorfromClass "/Game/BP/BP_Cursor.BP_Cursor_C" (Math|Transform|MakeTransform _vector "0, 0, 0" "0.400000,0.400000,0.010000") "Undefined" 0 0)
  (bind _distance (CallFunction|TwoPointDistance _position (Variables|/Game/BP/BP_BBCircleGameInstance.BP_BBCircleGameInstance_C|GetCenterPosition _as_bp_big_beautiful_circle_game_instance)))
  (Variables|/Game/BP/BP_BBCircleGameInstance.BP_BBCircleGameInstance_C|SetCenterDistance _as_bp_big_beautiful_circle_game_instance (+ (Math|Float|Absolute(Float) (- _distance (Variables|/Game/BP/BP_BBCircleGameInstance.BP_BBCircleGameInstance_C|GetRadius _as_bp_big_beautiful_circle_game_instance))) (Variables|/Game/BP/BP_BBCircleGameInstance.BP_BBCircleGameInstance_C|GetCenterDistance _as_bp_big_beautiful_circle_game_instance))))

(event Custom|InitialGameInstance
  (bind _asbp_big_beautiful_circle_game_instance (CallFunction|GetGameInstanceRef))
  (bind _output_get (Variables|Default|SetAs%20BP%20Big%20Beautiful%20Circle%20Game%20Instance _asbp_big_beautiful_circle_game_instance))
  (Variables|/Game/BP/BP_BBCircleGameInstance.BP_BBCircleGameInstance_C|SetAddCursor _output_get "")
  (Variables|/Game/BP/BP_BBCircleGameInstance.BP_BBCircleGameInstance_C|SetRemoveCursor _output_get "")
  (Variables|/Game/BP/BP_BBCircleGameInstance.BP_BBCircleGameInstance_C|SetCenterPosition _output_get "(X=0.500000,Y=0.500000)")
  (Variables|/Game/BP/BP_BBCircleGameInstance.BP_BBCircleGameInstance_C|SetRadius _output_get 2.5e+02)
  (Variables|/Game/BP/BP_BBCircleGameInstance.BP_BBCircleGameInstance_C|SetCenterDistance _output_get 0.0)
  (Variables|/Game/BP/BP_BBCircleGameInstance.BP_BBCircleGameInstance_C|SetScore _output_get 5e+04))

(event Custom|SpawnCheckPoint
  ;[1 1 1] SpawnCheckPoint
  (for (_array_element _array_index) (Variables|/Game/BP/BP_BBCircleGameInstance.BP_BBCircleGameInstance_C|GetCheckPointPosition (Variables|Default|GetAs%20BP%20Big%20Beautiful%20Circle%20Game%20Instance))
    (Game|SpawnActorfromClass "/Game/BP/BP_CheckPoint.BP_CheckPoint_C" (Math|Transform|MakeTransform _array_element "0, 0, 0" "0.500000,0.500000,0.030000") "Undefined" 0 _array_index 0)))

(event Custom|CheckCircle
  (bind _as_bp_big_beautiful_circle_game_instance (Variables|Default|GetAs%20BP%20Big%20Beautiful%20Circle%20Game%20Instance))
  (if (and (Utilities|Enum|Equal(Enum) (.state (Variables|/Game/BP/BP_BBCircleGameInstance.BP_BBCircleGameInstance_C|GetOneCursor _as_bp_big_beautiful_circle_game_instance)) "remove") (== (Variables|/Game/BP/BP_BBCircleGameInstance.BP_BBCircleGameInstance_C|GetBpEpDistance _as_bp_big_beautiful_circle_game_instance) 0.0))
    (bind _distance (CallFunction|TwoPointDistance (Variables|/Game/BP/BP_BBCircleGameInstance.BP_BBCircleGameInstance_C|GetAddCursor _as_bp_big_beautiful_circle_game_instance) (Variables|/Game/BP/BP_BBCircleGameInstance.BP_BBCircleGameInstance_C|GetRemoveCursor _as_bp_big_beautiful_circle_game_instance)))
    (bind _output_get (Variables|/Game/BP/BP_BBCircleGameInstance.BP_BBCircleGameInstance_C|SetBpEpDistance _as_bp_big_beautiful_circle_game_instance _distance))
    (Variables|/Game/BP/BP_BBCircleGameInstance.BP_BBCircleGameInstance_C|SetAddCursor _as_bp_big_beautiful_circle_game_instance "")
    (Development|PrintString (Utilities|String|ToString(Float) _output_get))
    (if (<= _output_get 5e+01)
      (if (Utilities|Array|Identical (Variables|/Game/BP/BP_BBCircleGameInstance.BP_BBCircleGameInstance_C|GetisCheckPointList _as_bp_big_beautiful_circle_game_instance) (Variables|/Game/BP/BP_BBCircleGameInstance.BP_BBCircleGameInstance_C|GetisThroughCheckPointList _as_bp_big_beautiful_circle_game_instance))
        (Variables|/Game/BP/BP_BBCircleGameInstance.BP_BBCircleGameInstance_C|SetisCircle _as_bp_big_beautiful_circle_game_instance true)
        (CallFunction|ShowScore)))))

(event Custom|Show%20Score
  (bind _as_bp_big_beautiful_circle_game_instance (Variables|Default|GetAs%20BP%20Big%20Beautiful%20Circle%20Game%20Instance))
  (Development|PrintString (Utilities|String|ToString(Float) (/ (- (Variables|/Game/BP/BP_BBCircleGameInstance.BP_BBCircleGameInstance_C|GetScore _as_bp_big_beautiful_circle_game_instance) (Variables|/Game/BP/BP_BBCircleGameInstance.BP_BBCircleGameInstance_C|GetCenterDistance _as_bp_big_beautiful_circle_game_instance)) 1e+03))))

(event EventBeginPlay
  (CallFunction|InitialGameInstance)
  (CallFunction|SpawnCheckPoint))

(event EventTick
  (params (DeltaSeconds :type Float%20%28single-precision%29))
  ;[1 1 1] Tick
  (bind _asbp_big_beautiful_circle_game_instance (CallFunction|GetGameInstanceRef))
  ;;[1 1 1] Check for differences from Before Cursror List
  (if (Utilities|Operators|EqualEqual (.position (Variables|/Game/BP/BP_BBCircleGameInstance.BP_BBCircleGameInstance_C|GetBeforeOneCursor _asbp_big_beautiful_circle_game_instance)) (.Position (Utilities|Struct|BreakF_Cursor (Variables|/Game/BP/BP_BBCircleGameInstance.BP_BBCircleGameInstance_C|GetOneCursor _asbp_big_beautiful_circle_game_instance))) 0.0)
    _
    (else
      (Variables|/Game/BP/BP_BBCircleGameInstance.BP_BBCircleGameInstance_C|SetBeforeOneCursor _asbp_big_beautiful_circle_game_instance (Variables|/Game/BP/BP_BBCircleGameInstance.BP_BBCircleGameInstance_C|GetOneCursor _asbp_big_beautiful_circle_game_instance))
      (CallFunction|SpawnCursor (Variables|/Game/BP/BP_BBCircleGameInstance.BP_BBCircleGameInstance_C|GetOneCursor _asbp_big_beautiful_circle_game_instance))))
  (CallFunction|CheckCircle))

(fn ConstructionScript)